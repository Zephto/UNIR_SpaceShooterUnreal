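; Player ship character for the space shooter, handling movement, firing and lives.
; Enhanced Input drives planar movement and spawns Ammo at FirePoint, with a timer-gated cooldown between shots.
; Actor overlaps use tags: Enemy removes a life with brief invincibility, Power adds one up to a cap.
; Losing the last life notifies ss_GameMode, plays explosion effects, then hides the actor and disables collision.
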(event `self.ReceiveBeginPlay`
  (bind _asplayer_controller (cast `PlayerController` (`self.GetController`)))
  (bind _returnvalue (pcsubsystem `EnhancedInputLocalPlayerSubsystem` _asplayer_controller))
  (`/Engine/EditorBlueprintResources/StandardMacros.IsValid` _returnvalue
    (:`Is Valid`
      (`EnhancedInputSubsystemInterface.AddMappingContext` _returnvalue "/Game/UNIR_SpaceShooter/Input/IMP_Player.IMP_Player" 0 (struct)))))

(event `self.ReceiveActorBeginOverlap`
  (params (OtherActor :type "Actor Object Reference"))
  (bind _tags (`Actor.Tags` OtherActor))
  (if (`KismetArrayLibrary.Array_Contains` _tags "Enemy")
    (`self.DamageActor`)
    (elif (`KismetArrayLibrary.Array_Contains` _tags "Power")
      (`self.AddLife`))))

(event `EnhancedInput|/Game/UNIR_SpaceShooter/Input/BP_InputMove`
  (params (ActionValue :type "Vector2D Structure") (ElapsedSeconds :type "Float (double-precision)") (TriggeredSeconds :type "Float (double-precision)") (InputAction :type "InputAction Object Reference" :default "/Game/UNIR_SpaceShooter/Input/BP_InputMove.BP_InputMove"))
  (:`Triggered`
    (`self.AddMovementInput` (`self.GetActorRightVector`) ActionValue_X)
    (`self.AddMovementInput` (`self.GetActorForwardVector`) ActionValue_Y)))

(event `EnhancedInput|/Game/UNIR_SpaceShooter/Input/BP_InputFire`
  (params (ActionValue :type Boolean) (ElapsedSeconds :type "Float (double-precision)") (TriggeredSeconds :type "Float (double-precision)") (InputAction :type "InputAction Object Reference" :default "/Game/UNIR_SpaceShooter/Input/BP_InputFire.BP_InputFire"))
  (:`Triggered`
    (if (`self.CanFire`)
      (`self.DoFire`)
      (set `self.CanFire` false)
      (`KismetSystemLibrary.K2_SetTimerDelegate` (delegate `UpdateFire`) (`self.FireDelay`))
      (`GameplayStatics.PlaySound2D` "/Game/StarterContent/Audio/Explosion01.Explosion01" 0.5 0.5 0.0 null null))))

(event `UpdateFire`
  (set `self.CanFire` true))

(event `DamageActor`
  (if (not (`self.TemporalInvencible`))
    (set `self.TemporalInvencible` true)
    (bind _output_get (set `self.Lifes` (- (`self.Lifes`) 1)))
    (if (== _output_get 0)
      (bind _asss_game_mode (cast `/Game/UNIR_SpaceShooter/ss_GameMode` (`GameplayStatics.GetGameMode`)))
      (`/Game/UNIR_SpaceShooter/ss_GameMode.PlayerDead` _asss_game_mode)
      (`GameplayStatics.SpawnEmitterAtLocation` "/Game/StarterContent/Particles/P_Explosion.P_Explosion" (`self.K2_GetActorLocation`))
      (`GameplayStatics.PlaySound2D` "/Game/StarterContent/Audio/Explosion02.Explosion02" 1.0 1.0 0.0 null null)
      (`KismetSystemLibrary.Delay` 0.2)
      (`self.SetActorHiddenInGame` true)
      (`self.SetActorEnableCollision` false)
      (else
        (`KismetSystemLibrary.Delay` 0.5)
        (set `self.TemporalInvencible` false)))))

(event `AddLife`
  (bind _output_get (set `self.Lifes` (+ (`self.Lifes`) 1)))
  (if (>= _output_get 3)
    (set `self.Lifes` 3)))

(fn `DoFire`
  (`|SpawnActorFromClass` (`self.Ammo`) (`SceneComponent.K2_GetComponentToWorld` (`self.FirePoint`)) "Undefined" "MultiplyWithRoot" null null))

(fn `UserConstructionScript`)