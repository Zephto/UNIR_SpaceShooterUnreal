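; BP_SS_AmmoPlayer is the player's projectile in the space shooter, moving along its forward vector every Tick at Speed, without sweep.
; On overlap it ignores actors tagged PlayerWall and self-destructs after a short delay on those tagged Wall.
; Any other actor also triggers an explosion emitter at that actor's location and a sound before the same delayed self-destruction, with no damage applied here.
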(event `self.ReceiveActorBeginOverlap`
  (params (OtherActor :type "Actor Object Reference"))
  (bind _tags (`Actor.Tags` OtherActor))
  (if (`KismetArrayLibrary.Array_Contains` _tags "Wall")
    (`KismetSystemLibrary.Delay` 0.1 :!label _label)
    (`self.K2_DestroyActor`)
    (elif (not (`KismetArrayLibrary.Array_Contains` _tags "PlayerWall"))
      (`GameplayStatics.SpawnEmitterAtLocation` "/Game/StarterContent/Particles/P_Explosion.P_Explosion" (`self.K2_GetActorLocation` OtherActor))
      (`GameplayStatics.PlaySound2D` "/Game/StarterContent/Audio/Explosion02.Explosion02" 1.0 1.0 0.0 null null)
      (goto _label))))

(event `self.ReceiveTick`
  (params (DeltaSeconds :type "Float (single-precision)"))
  (`self.K2_SetActorLocation` (+ (`self.K2_GetActorLocation`) (* (`self.GetActorForwardVector`) (* DeltaSeconds (`self.Speed`))))))

(fn `UserConstructionScript`)