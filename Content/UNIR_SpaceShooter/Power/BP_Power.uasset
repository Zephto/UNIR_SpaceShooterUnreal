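; BP_Power is a power pickup actor for the space shooter that flies in a straight line until it hits a wall or the player.
; BeginPlay caches the forward vector, and Tick moves the actor along it by Speed scaled by delta time, without sweeping.
; Overlaps are filtered by actor tag: PlayerBody plays a select sound, and both it and Wall destroy the pickup after a short delay.
; No power effect is applied in this Blueprint.
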(event `self.ReceiveActorBeginOverlap`
  (params (OtherActor :type "Actor Object Reference"))
  (bind _tags (`Actor.Tags` OtherActor))
  (if (`KismetArrayLibrary.Array_Contains` _tags "Wall")
    (`KismetSystemLibrary.Delay` 0.2 :!label _label)
    (`self.K2_DestroyActor`)
    (elif (`KismetArrayLibrary.Array_Contains` _tags "PlayerBody")
      (`GameplayStatics.PlaySound2D` "/Game/UNIR_SpaceShooter/sound/1-07__Select.1-07__Select" 1.0 1.0 0.0 null null)
      (goto _label))))

(event `self.ReceiveBeginPlay`
  (set `self.MovementVector` (`self.GetActorForwardVector`)))

(event `self.ReceiveTick`
  (params (DeltaSeconds :type "Float (single-precision)"))
  (`self.K2_SetActorLocation` (+ (* (* DeltaSeconds (`self.Speed`)) (`self.MovementVector`)) (`self.K2_GetActorLocation`))))

(fn `UserConstructionScript`)