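; Spawner actor for the space shooter that periodically creates enemies at a random SceneComponent of its own tagged SpawnPoint.
; A looping timer spawns only when the GameMode's Level is not a multiple of 3.
; A random index below Level, clamped by MaxNumEnemies, selects BP_EnemyBase_H or BP_EnemyBase_HF.
; Each enemy's destroy event decrements SpawnTime, but the running timer is never reset with the new value.
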(event `self.ReceiveBeginPlay`
  (`KismetSystemLibrary.K2_SetTimerDelegate` (delegate `Spawn`) (`self.SpawnTime`) true)
  (bind _asss_game_mode (cast `/Game/UNIR_SpaceShooter/ss_GameMode` (`GameplayStatics.GetGameMode`)))
  (set `self.As Ss Game Mode` _asss_game_mode))

(event `Spawn`
  (if (`KismetMathLibrary.Conv_IntToBool` (mod (`/Game/UNIR_SpaceShooter/ss_GameMode.Level` (`self.As Ss Game Mode`)) 3))
    (bind _newparam (`self.SpawnEnemy`))
    (add `/Game/UNIR_SpaceShooter/Enemies/BP_EnemyBase.OnEnemyDestroy` _newparam (delegate `EnemyDestroyed`))))

(event `EnemyDestroyed`
  (set `self.SpawnTime` (- (`self.SpawnTime`) 1.0)))

(fn `GetClassToSpawn`
  (params (Value :type Integer))
  (returns (Class :type "/Game/UNIR_SpaceShooter/Enemies/BP_EnemyBase Class Reference"))
  (return (select `int` (`KismetMathLibrary.Clamp` Value 0 (- (`self.MaxNumEnemies`) 1)) :`0` "/Game/UNIR_SpaceShooter/Enemies/BP_EnemyBase_H.BP_EnemyBase_H_C" :`1` "/Game/UNIR_SpaceShooter/Enemies/BP_EnemyBase_HF.BP_EnemyBase_HF_C" :!type "/Game/UNIR_SpaceShooter/Enemies/BP_EnemyBase Class Reference")))

(fn `SpawnEnemy`
  (returns (NewParam :type "/Game/UNIR_SpaceShooter/Enemies/BP_EnemyBase Object Reference"))
  (locals (NewLocalVar :type "/Game/UNIR_SpaceShooter/ss_GameMode Object Reference"))
  (bind _returnvalue (`self.GetComponentsByTag` "/Script/Engine.SceneComponent" "SpawnPoint"))
  (bind _class (`self.GetClassToSpawn` (`KismetMathLibrary.RandomInteger` (`/Game/UNIR_SpaceShooter/ss_GameMode.Level` (`self.As Ss Game Mode`)))))
  (bind _returnvalue_2 (`|SpawnActorFromClass` _class (`SceneComponent.K2_GetComponentToWorld` (`|GetArrayItem` _returnvalue (`KismetMathLibrary.RandomInteger` (`KismetArrayLibrary.Array_Length` _returnvalue)))) "Undefined" "MultiplyWithRoot" null null))
  (bind _asbp_enemy_base (cast `/Game/UNIR_SpaceShooter/Enemies/BP_EnemyBase` _returnvalue_2))
  (return _asbp_enemy_base))

(fn `UserConstructionScript`)