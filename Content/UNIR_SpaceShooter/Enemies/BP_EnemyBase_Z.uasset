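; Enemy Blueprint for the space shooter that overrides the movement vector on top of its parent class's behavior.
; BeginPlay calls the parent, then sets MovementVector to the actor's right vector.
; Tick calls the parent, then zeroes MovementVector, so the initial direction lasts only until the first Tick finishes.
; An unconnected sine calculation is left unused, and the overlap event is disabled.
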(event `self.ReceiveBeginPlay`
  (`parent.ReceiveBeginPlay`)
  (set `self.MovementVector` (`self.GetActorRightVector`)))

(event `self.ReceiveTick`
  (params (DeltaSeconds :type "Float (single-precision)"))
  (`parent.ReceiveTick` DeltaSeconds)
  (set `self.MovementVector` (0.0 0.0 0.0)))

(fn `UserConstructionScript`
  (`parent.UserConstructionScript`))