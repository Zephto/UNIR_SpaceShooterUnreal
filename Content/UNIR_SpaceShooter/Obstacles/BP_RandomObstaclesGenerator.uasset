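; BP_RandomObstaclesGenerator is a space shooter spawner that periodically creates random obstacles during play.
; After a short delay, BeginPlay starts a looping SpawnTime timer and caches the game mode.
; Each tick of that timer spawns one of four obstacle classes, limited by MaxNumEnemies, at a random component tagged SpawnPoint.
; An EnemyDestroyed handler lowers SpawnTime, but its binding never runs and the timer is not reset.
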(event `self.ReceiveBeginPlay`
  (`KismetSystemLibrary.Delay` 1.0)
  (`KismetSystemLibrary.K2_SetTimerDelegate` (delegate `Spawn`) (`self.SpawnTime`) true)
  (bind _asss_game_mode (cast `/Game/UNIR_SpaceShooter/ss_GameMode` (`GameplayStatics.GetGameMode`)))
  (set `self.As Ss Game Mode` _asss_game_mode))

(event `Spawn`
  (`self.SpawnEnemy`))

(event `EnemyDestroyed`
  (set `self.SpawnTime` (- (`self.SpawnTime`) 1.0)))

(fn `GetClassToSpawn`
  (params (Value :type Integer))
  (returns (Class :type "/Game/UNIR_SpaceShooter/Obstacles/BP_ObstacleBase Class Reference"))
  (return (select `int` (`KismetMathLibrary.Clamp` Value 0 (`self.MaxNumEnemies`)) :`0` "/Game/UNIR_SpaceShooter/Obstacles/BP_Obstacle_2.BP_Obstacle_2_C" :`1` "/Game/UNIR_SpaceShooter/Obstacles/BP_Obstacle_3.BP_Obstacle_3_C" :`2` "/Game/UNIR_SpaceShooter/Obstacles/BP_Obstacle_4.BP_Obstacle_4_C" :`3` "/Game/UNIR_SpaceShooter/Obstacles/BP_Obstacle_5.BP_Obstacle_5_C" :!type "/Game/UNIR_SpaceShooter/Obstacles/BP_ObstacleBase Class Reference")))

(fn `SpawnEnemy`
  (bind _returnvalue (`self.GetComponentsByTag` "/Script/Engine.SceneComponent" "SpawnPoint"))
  (bind _class (`self.GetClassToSpawn` (`KismetMathLibrary.RandomInteger` (`self.MaxNumEnemies`))))
  (`|SpawnActorFromClass` _class (`SceneComponent.K2_GetComponentToWorld` (`|GetArrayItem` _returnvalue (`KismetMathLibrary.RandomInteger` (`KismetArrayLibrary.Array_Length` _returnvalue)))) "Undefined" "MultiplyWithRoot" null null)
  (return))

(fn `UserConstructionScript`)