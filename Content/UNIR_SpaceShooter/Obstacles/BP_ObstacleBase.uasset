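; BP_ObstacleBase is the base obstacle actor for the space shooter, moving in a straight line until it reaches a wall.
; On BeginPlay it captures its forward vector as the movement direction.
; Each tick it offsets its location along that vector by Speed scaled by delta time, without sweeping.
; Overlapping an actor tagged Wall destroys it after a short delay.
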(event `self.ReceiveActorBeginOverlap`
  (params (OtherActor :type "Actor Object Reference"))
  (if (`KismetArrayLibrary.Array_Contains` (`Actor.Tags` OtherActor) "Wall")
    (`KismetSystemLibrary.Delay` 0.2)
    (`self.K2_DestroyActor`)))

(event `self.ReceiveBeginPlay`
  (set `self.MovementVector` (`self.GetActorForwardVector`)))

(event `self.ReceiveTick`
  (params (DeltaSeconds :type "Float (single-precision)"))
  (`self.K2_SetActorLocation` (+ (* (* DeltaSeconds (`self.Speed`)) (`self.MovementVector`)) (`self.K2_GetActorLocation`))))

(fn `UserConstructionScript`)