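; BP_SS_HUD manages the on-screen HUD for the space shooter game.
; On BeginPlay it creates a BP_UserWidget for player 0, adds it to the viewport, and caches the BP_SS_Character and ss_GameMode.
; Every Tick it pushes the game mode's progress and the character's lives to the widget.
; A PlayerKilled event forwards the player's death to the widget.
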(event `self.ReceiveBeginPlay`
  (bind _returnvalue (`GameplayStatics.GetPlayerController` 0))
  (`/Engine/EditorBlueprintResources/StandardMacros.IsValid` _returnvalue
    (:`Is Valid`
      (bind _returnvalue_2 (`|CreateWidget` "/Game/UNIR_SpaceShooter/HUD/BP_UserWidget.BP_UserWidget_C" _returnvalue))
      (bind _output_get (set `self.GameWidget` _returnvalue_2))
      (`UserWidget.AddToViewport` _output_get 0)
      (bind _asbp_ss_character (cast `/Game/UNIR_SpaceShooter/Players/BP_SS_Character` (`GameplayStatics.GetPlayerCharacter` 0)))
      (set `self.m_PlayerCharacter` _asbp_ss_character)
      (bind _asss_game_mode (cast `/Game/UNIR_SpaceShooter/ss_GameMode` (`GameplayStatics.GetGameMode`)))
      (set `self.Ss_Game_Mode` _asss_game_mode))))

(event `self.ReceiveTick`
  (params (DeltaSeconds :type "Float (single-precision)"))
  (`/Game/UNIR_SpaceShooter/HUD/BP_UserWidget.UpdateWidget` (`self.GameWidget`) (`/Game/UNIR_SpaceShooter/ss_GameMode.Progress` (`self.Ss_Game_Mode`)) (`/Game/UNIR_SpaceShooter/Players/BP_SS_Character.Lifes` (`self.m_PlayerCharacter`))))

(event `PlayerKilled`
  (`/Game/UNIR_SpaceShooter/HUD/BP_UserWidget.PlayerKilled` (`self.GameWidget`)))

(fn `UserConstructionScript`)